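; BP_Noglo is an interactive lift prop with a rope, toggled up or down with E while input is enabled by its trigger box.
; Each toggle plays a skeletal animation and sound, ignoring animation changes while one plays; lifting up first plays the down sound and waits.
; The Rope timeline runs forward or reverse, scrolling a dynamic rope material through OffsetV.
; Tick hides the UI during animation.
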(event `self.ReceiveBeginPlay`
  (bind _returnvalue (`PrimitiveComponent.CreateDynamicMaterialInstance` (`self.SKM_Noglo`) 0 "/Game/KTInteractionPropVol1/Material/M_Rope.M_Rope" "OffsetV"))
  (set `self.Mi_Rope` _returnvalue))

(event `self.ReceiveTick`
  (params (DeltaSeconds :type "Float (single-precision)"))
  (if (`SkeletalMeshComponent.IsPlaying` (`self.SKM_Noglo`))
    (`self.SetUI` true)
    (else
      (`self.SetUI` false))))

(event `Key|E`
  (params (Key :type "Key Structure"))
  (bind _skm_noglo (`self.SKM_Noglo`))
  (:`Pressed`
    (if (`self.IsDown`)
      (`GameplayStatics.PlaySoundAtLocation` "/Game/KTInteractionPropVol1/Sound/Sound_Noglo_LiftDown.Sound_Noglo_LiftDown" (0.0 0.0 0.0) (struct) 1.0 1.0 0.0 null null null null)
      (`KismetSystemLibrary.Delay` 4.0))
    (if (`SkeletalMeshComponent.IsPlaying` _skm_noglo)
      _
      (elif (`self.IsDown`)
        (`SkeletalMeshComponent.PlayAnimation` _skm_noglo "/Game/KTInteractionPropVol1/Animation/ANIM_Noglo_LiftUp.ANIM_Noglo_LiftUp" false)
        (`GameplayStatics.PlaySoundAtLocation` "/Game/KTInteractionPropVol1/Sound/Sound_Noglo_LiftUp.Sound_Noglo_LiftUp" (0.0 0.0 0.0) (struct) 1.0 1.0 0.0 null null null null)
        (set `self.IsDown` false)
        (bind (_direction _liftup) (`Timeline|Rope` :!label _label)
          (:`Update`
            (`MaterialInstanceDynamic.SetScalarParameterValue` (`self.Mi_Rope`) "OffsetV" _liftup)))
        (else
          (`SkeletalMeshComponent.PlayAnimation` _skm_noglo "/Game/KTInteractionPropVol1/Animation/ANIM_Noglo_LiftDown.ANIM_Noglo_LiftDown" false)
          (`GameplayStatics.PlaySoundAtLocation` "/Game/KTInteractionPropVol1/Sound/Sound_Noglo_LiftDown.Sound_Noglo_LiftDown" (0.0 0.0 0.0) (struct) 1.0 1.0 0.0 null null null null)
          (set `self.IsDown` true)
          (goto _label :!via `Reverse`))))))

(event `self.Trigger Box R.OnComponentBeginOverlap`
  (params (OverlappedComponent :type "PrimitiveComponent Object Reference") (OtherActor :type "Actor Object Reference") (OtherComp :type "PrimitiveComponent Object Reference") (OtherBodyIndex :type Integer) (bFromSweep :type Boolean) (SweepResult :type "HitResult Structure (by ref)"))
  (`self.EnableInput` (`GameplayStatics.GetPlayerController` 0)))

(event `self.Trigger Box R.OnComponentEndOverlap`
  (params (OverlappedComponent :type "PrimitiveComponent Object Reference") (OtherActor :type "Actor Object Reference") (OtherComp :type "PrimitiveComponent Object Reference") (OtherBodyIndex :type Integer))
  (`self.DisableInput` (`GameplayStatics.GetPlayerController` 0)))

(fn `SetUI`
  (params (Hidden :type Boolean))
  (`SceneComponent.SetHiddenInGame` (`self.UI`) Hidden false))

(fn `UserConstructionScript`)